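; BP_AI_Greystone is an AI character Blueprint for Greystone with an unfinished combat behavior loop.
; BeginPlay calls CombatStart, which creates a looping timer for CombatLogic, then immediately pauses and clears it.
; CombatLogic gates on a valid, living target, state flags and depleted attack counts.
; Its final sequence is empty, with only a comment naming attack recharge and strafing.
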(event `self.ReceiveBeginPlay`
  (`self.CombatStart`))

(event `CombatStart`
  (bind _returnvalue (`KismetSystemLibrary.K2_SetTimerDelegate` (delegate `CombatLogic`) 0.2 true))
  (bind _output_get (set `self.CombatStartHandle` _returnvalue))
  (`KismetSystemLibrary.K2_PauseTimerHandle` _output_get)
  (`KismetSystemLibrary.K2_ClearAndInvalidateTimerHandle` _output_get))

(event `CombatLogic`
  (bind _target (`self.Target`)
    (:`then`
      (bind _alive_ (message `/Game/_MCAI/Data/BPI_Combat.INT_isAlive?` _target))
      (if (and _alive_ (not (`self.Dead`)) (`self.AllowBehave?`) (`self.EnableTick`))
        (if (<= (`self.AttackCounts`) 0)
          ;[1 1 1] 1. Recharge Attack counts     2. Start to Strafe
          (`|ExecutionSequence`))))
    (:`else`)))

(fn `UserConstructionScript`)